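; BP_STUBaseCharacter is a player character Blueprint that adds walk and run speed switching.
; BeginPlay sets the movement component's max walk speed to the walk value.
; Pressing Left Shift switches to run speed only if IsMovingForward is true at that moment, and releasing it restores walk speed.
; The key is bound directly in the event graph, and IsMovingForward is only read here, never set.
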(event EventBeginPlay
  (Variables|/Script/Engine.CharacterMovementComponent|SetMaxWalkSpeed (Variables|Character|GetCharacterMovement) (Variables|Default|GetWalkSpeed)))

(event Collision|EventActorBeginOverlap
  (params (OtherActor :type Actor%20Object%20Reference)))

(event EventTick
  (params (DeltaSeconds :type Float%20%28single-precision%29)))

(event Input|KeyboardEvents|LeftShift
  (params (Key :type Key%20Structure :default "None"))
  (bind _charactermovement (Variables|Character|GetCharacterMovement))
  (:Pressed
    (if (Variables|Default|GetIsMovingForward)
      (Variables|Default|SetIsRunning true)
      (Variables|/Script/Engine.CharacterMovementComponent|SetMaxWalkSpeed _charactermovement (Variables|Default|GetRunSpeer))))
  (:Released
    (if (Variables|Default|GetIsRunning)
      (Variables|Default|SetIsRunning false)
      (Variables|/Script/Engine.CharacterMovementComponent|SetMaxWalkSpeed _charactermovement (Variables|Default|GetWalkSpeed)))))

(fn ConstructionScript)